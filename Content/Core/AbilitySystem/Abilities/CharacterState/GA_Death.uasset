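; Death gameplay ability that, on a received hit event, plays a death montage and turns the character into a ragdoll.
; It fires a hit gameplay cue and applies a brief root-motion impulse away from the damage applier.
; An EnableRagdoll gameplay event disables capsule collision and starts mesh physics.
; SetMontageToPlay selects a directional death montage, but playback uses the hard-coded forward montage.
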(event Ability|EventActivateAbility
  (|CallParentFunction) ; This node is disabled and will not be called.\nDrag off pins to build functionality.
)

(event Ability|EventOnEndAbility
  (params (bWasCancelled :type Boolean))
  (|CallParentFunction bWasCancelled) ; This node is disabled and will not be called.\nDrag off pins to build functionality.
)

(event EventHitEventReceived
  (params (GameplayEventData :type Gameplay%20Event%20Data%20Structure%20%28by%20ref%29))
  (|CallParentFunction GameplayEventData)
  (|PlayMontageandWaitProxy "None" "/Game/Animation/Death/AM_Death_Forward.AM_Death_Forward" 1.0 "None" true 1.0 0.0 true
    (:then
      (Utilities|FlowControl|Sequence
        (:then_0
          (Class|GameplayAbility|ExecuteGameplayCuewithParams "(TagName=\"GameplayCue.HitReceived\")" (Ability|GameplayCue|MakeGameplayCueParameters 0.0 0.0 (Variables|Default|GetCachedEffectContext)))
          (Ability|Tasks|WaitGameplayEvent "(TagName=\"Event.Combat.EnableRagdoll\")" 0 true
            (:EventReceived
              (CallFunction|HandleRagdoll))))
        (:then_1
          (Ability|Tasks|ApplyRootMotionConstantForce "None" (* (Variables|Default|GetDirToDamageApplierXY) -1) (.DeathImpulseStrength (Utilities|Struct|BreakTDWDamageSpec (Variables|Default|GetCachedDamageSpec))) 0.1 true 0 "MaintainLastRootMotionVelocity" "0, 0, 0" 0.0 true))))))

(fn SetMontagetoPlay
  (params (InMontage :type Anim%20Montage%20Object%20Reference))
  (|CallParentFunction (.Value (Utilities|Map|Find (Utilities|Struct|BreakDirectionMontageSpec (Class|TDWCharacterAssets|GetDeathMontages (Class|TDWCharacterBase|GetCharacterAssets (Class|TDWGameplayAbilityBase|GetBaseCharacter)))) (CallFunction|CalculateDirectiontoApplier)))))

(fn HandleRagdoll
  (Utilities|FlowControl|Sequence
    (:then_0
      (Collision|SetCollisionEnabled (Variables|/Script/Engine.Character|GetCapsuleComponent (Class|TDWGameplayAbilityBase|GetBaseCharacter)) "NoCollision"))
    (:then_1
      (bind _output_get (LocalVariables|SetMesh (Variables|/Script/Engine.Character|GetMesh (Class|TDWGameplayAbilityBase|GetBaseCharacter))))
      (Collision|SetCollisionProfileName _output_get "Ragdoll" true :!class /Script/Engine.PrimitiveComponent)
      (Physics|SetEnableGravity (LocalVariables|GetMesh) true)
      (Physics|SetSimulatePhysics (LocalVariables|GetMesh) true)
      (Collision|SetCollisionEnabled (LocalVariables|GetMesh) "QueryAndPhysics")
      (Collision|SetCollisionResponsetoChannel (LocalVariables|GetMesh) "ECC_WorldStatic" "ECR_Block")
      (Collision|SetCollisionResponsetoChannel (LocalVariables|GetMesh) "ECC_WorldDynamic" "ECR_Block"))))