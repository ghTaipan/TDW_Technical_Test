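; Hit reaction gameplay ability that plays a directional montage when a character receives a hit event.
; It picks the montage from the character's assets by the cached damage spec's react type and the direction to the damage applier.
; Each hit also applies a brief additive root motion push away from the applier and fires the HitReceived gameplay cue.
; A flag keeps the ability alive when a new hit interrupts the current montage.
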(event Ability|EventActivateAbility
  (|CallParentFunction))

(event Ability|EventOnEndAbility
  (params (bWasCancelled :type Boolean))
  (|CallParentFunction bWasCancelled)
  (Variables|Default|SetbHitReactEventReceived false))

(event EventHitEventReceived
  (params (GameplayEventData :type Gameplay%20Event%20Data%20Structure%20%28by%20ref%29))
  (|CallParentFunction GameplayEventData)
  (Variables|Default|SetbHitReactEventReceived true)
  (|PlayMontageandWaitProxy "None" (Class|TDWGameplayAbilityBase|GetMontagetoPlay) 1.0 "None" true 1.0 0.0 true
    (:then
      (Variables|Default|SetbHitReactEventReceived false)
      (Ability|Tasks|ApplyRootMotionConstantForce "None" (* (Variables|Default|GetDirToDamageApplierXY) -1) (.HitImpulseStrength (Utilities|Struct|BreakTDWDamageSpec (Variables|Default|GetCachedDamageSpec))) 0.1 true 0 "MaintainLastRootMotionVelocity" "0, 0, 0" 0.0 true
        (:then
          (Class|GameplayAbility|ExecuteGameplayCuewithParams "(TagName=\"GameplayCue.HitReceived\")" (Ability|GameplayCue|MakeGameplayCueParameters 0.0 1.0 (Variables|Default|GetCachedEffectContext))))))
    (:OnCompleted
      (Ability|EndAbility))
    (:OnInterrupted
      (if (not (Variables|Default|GetbHitReactEventReceived)) :!label _label
        (Ability|EndAbility)))
    (:OnCancelled
      (goto _label))))

(fn SetMontagetoPlay
  (params (InMontage :type Anim%20Montage%20Object%20Reference))
  (|CallParentFunction (.Value (Utilities|Map|Find (Utilities|Struct|BreakDirectionMontageSpec (.Value (Utilities|Map|Find (Class|TDWCharacterAssets|GetHitReactMontages (Class|TDWCharacterBase|GetCharacterAssets (Class|TDWGameplayAbilityBase|GetBaseCharacter))) (.HitReactType (Utilities|Struct|BreakTDWDamageSpec (Variables|Default|GetCachedDamageSpec)))))) (CallFunction|CalculateDirectiontoApplier)))))