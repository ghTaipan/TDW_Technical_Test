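; Base Gameplay Ability for character states that react to hits, listening for the Event.Combat.HitReact gameplay event once activated.
; Each event caches the effect context and its damage spec, then calls SetMontageToPlay.
; Helper functions classify the damage applier's position relative to the receiver's forward vector into four clock-named directions, using a flattened dot product and cross-product sign.
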(event Custom|HitEventReceived
  (params (GameplayEventData :type Gameplay%20Event%20Data%20Structure%20%28by%20ref%29))
  (bind _output_get (Variables|Default|SetCachedEffectContext (.ContextHandle (Utilities|Struct|BreakGameplayEventData GameplayEventData))))
  (Variables|Default|SetCachedDamageSpec (Class|TDWAbilitySystemBlueprintLibrary|GetDamageSpec _output_get))
  (Class|TDWGameplayAbilityBase|SetMontagetoPlay))

(event Ability|EventActivateAbility
  (bind _payload (Ability|Tasks|WaitGameplayEvent "(TagName=\"Event.Combat.HitReact\")" 0 (Variables|Default|GetbTriggerHİtEventOnce))
    (:EventReceived
      (CallFunction|HitEventReceived _payload))))

(event Ability|EventOnEndAbility
  (params (bWasCancelled :type Boolean)))

(fn GetDirectionfromXYDot
  (params (VectorA :type Vector) (VectorB :type Vector))
  (bind _output_get (LocalVariables|SetDotResult (Math|Vector|DotProduct (Math|Vector|MakeVector (.x VectorA) (.y VectorA) 0.0) (Math|Vector|MakeVector (.x VectorB) (.y VectorB) 0.0))))
  (if (>= _output_get 0.5)
    (return "Clock12")
    (elif (<= (LocalVariables|GetDotResult) -0.5)
      (return "Clock3")
      (elif (> (.Z (Math|Vector|BreakVector (Math|Vector|CrossProduct VectorA VectorB))) 0.0)
        (return "Clock9")
        (else
          (return "Clock6"))))))

(fn CalculateDirectiontoApplier
  (bind _cacheddamagespec (Variables|Default|GetCachedDamageSpec))
  (bind (_damageapplier _damagereceiver) (Utilities|Struct|BreakTDWDamageSpec _cacheddamagespec))
  (bind _returnvalue (Transformation|GetActorLocation _damageapplier))
  (bind _returnvalue_2 (Transformation|GetActorLocation _damagereceiver))
  (Utilities|FlowControl|Sequence
    (:then_0
      (Variables|Default|SetDirToDamageApplierXY (Math|Vector|Normalize (- (Math|Vector|MakeVector (.x _returnvalue) (.y _returnvalue) 0.0) (Math|Vector|MakeVector (.x _returnvalue_2) (.y _returnvalue_2) 0.0))))
      (LocalVariables|SetRecieverForward (Transformation|GetActorForwardVector _damagereceiver)))
    (:then_1
      (return (CallFunction|GetDirectionfromXYDot (LocalVariables|GetRecieverForward) (Variables|Default|GetDirToDamageApplierXY))))))