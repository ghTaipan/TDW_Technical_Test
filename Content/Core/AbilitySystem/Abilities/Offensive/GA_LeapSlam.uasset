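; Leap Slam offensive gameplay ability that plays an attack montage and deals damage on hit.
; On successful commit, it plays the montage mapped to the LeapSlam tag in the character's skill assets, scaling play rate by a character attribute with a default fallback.
; Hit-detected gameplay events pass their context to apply the damage effect spec.
; The ability ends when the montage completes or breaks off, and cancels if commit fails.
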(event Ability|EventActivateAbility
  (bind _returnvalue (Ability|CommitAbility))
  (if _returnvalue
    (CallFunction|SetMontagetoPlay)
    (|PlayMontageandWaitProxy "None" (Class|TDWGameplayAbilityBase|GetMontagetoPlay) (CallFunction|GetAttackSpeed) "None" true 1.0 0.0 true
      (:then
        (bind _payload (Ability|Tasks|WaitGameplayEvent "(TagName=\"Event.Combat.HitDetected\")" 0)
          (:EventReceived
            (Class|TDWGameplayAbilityBase|ApplyDamageEffectfromSpec (.ContextHandle (Utilities|Struct|BreakGameplayEventData _payload))))))
      (:OnCompleted
        (Ability|EndAbility :!label _label))
      (:OnInterrupted
        (goto _label))
      (:OnCancelled
        (goto _label)))
    (else
      (Ability|CancelAbility))))

(event Ability|EventOnEndAbility
  (params (bWasCancelled :type Boolean)))

(fn ApplyDamage)

(fn SetMontagetoPlay
  (params (InMontage :type Anim%20Montage%20Object%20Reference))
  (|CallParentFunction (.Value (Utilities|Map|Find (Class|TDWCharacterAssets|GetSkillMontages (Class|TDWCharacterBase|GetCharacterAssets (Class|TDWGameplayAbilityBase|GetBaseCharacter))) "(TagName=\"Ability.Combat.Offensive.LeapSlam\")"))))

(fn GetAttackSpeed
  (bind _returnvalue (Class|TDWGameplayAbilityBase|GetBaseCharacter))
  (bind (_bsuccessfullyfoundattribute _returnvalue_2) (Ability|Attribute|GetFloatAttribute _returnvalue "(AttributeName=\"CurrentAttackSpeed\",Attribute=/Script/TDW_Technical_Test.TDWAttackSpeedAttributeSet:CurrentAttackSpeed,AttributeOwner=\"/Script/CoreUObject.Class'/Script/TDW_Technical_Test.TDWAttackSpeedAttributeSet'\")"))
  (return (Math|Float|SelectFloat _returnvalue_2 1.0 _bsuccessfullyfoundattribute)))