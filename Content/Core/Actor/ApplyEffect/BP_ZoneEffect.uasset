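; BP_ZoneEffect is a box trigger zone that applies a configurable Gameplay Effect to overlapping actors that have an Ability System Component.
; On begin overlap it async-loads the effect class, applies it at level 1 and stores the handle in a single variable, overwritten on each application.
; On end overlap it optionally removes the effect using that handle.
; The construction script displays the effect label on a text render.
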(event OnComponentBeginOverlap(Box)
  (params (OverlappedComponent :type Primitive%20Component%20Object%20Reference) (OtherActor :type Actor%20Object%20Reference) (OtherComp :type Primitive%20Component%20Object%20Reference) (OtherBodyIndex :type Integer) (bFromSweep :type Boolean) (SweepResult :type Hit%20Result%20Structure%20%28by%20ref%29))
  (bind _returnvalue (Ability|GetAbilitySystemComponent OtherActor))
  (Utilities|IsValid _returnvalue
    (:Is%20Valid
      (bind _class (Utilities|AsyncLoadClassAsset (Variables|Config|GetEffectType))
        (:Completed
          (bind _asgameplay_effect (Utilities|Casting|CastToGameplayEffectClass _class))
          (bind _returnvalue_2 (GameplayEffects|ApplyGameplayEffectToSelf _returnvalue _asgameplay_effect 1.0 (GameplayEffects|MakeEffectContext _returnvalue)))
          (Variables|Default|SetEffectHandle _returnvalue_2))))))

(event OnComponentEndOverlap(Box)
  (params (OverlappedComponent :type Primitive%20Component%20Object%20Reference) (OtherActor :type Actor%20Object%20Reference) (OtherComp :type Primitive%20Component%20Object%20Reference) (OtherBodyIndex :type Integer))
  (bind _returnvalue (Ability|GetAbilitySystemComponent OtherActor))
  (if (and (Variables|Default|GetbRemoveOnEndOverlap) (Utilities|IsValid _returnvalue))
    (GameplayEffects|RemoveActiveGameplayEffect _returnvalue (Variables|Default|GetEffectHandle) -1)))

(event EventBeginPlay)

(event Collision|EventActorBeginOverlap
  (params (OtherActor :type Actor%20Object%20Reference)))

(event EventTick
  (params (DeltaSeconds :type Float%20%28single-precision%29)))

(fn ConstructionScript
  (Rendering|Components|TextRender|SetText (Variables|Default|GetTextRender) (Variables|Config|GetEffectText)))